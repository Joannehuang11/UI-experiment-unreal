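; Scene capture camera actor for the HUD mini map that renders a top-down view centered on the player character.
; On BeginPlay it moves its CaptureComponent2D to the player's location.
; Each tick it places the capture at the player's X and Y at a fixed world height, pointing straight down and yawed with the character so the view rotates with the player's facing.
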(event `self.ReceiveBeginPlay`
  (`SceneComponent.K2_SetWorldLocation` (`self.CaptureComponent2D`) (`self.K2_GetActorLocation` (`GameplayStatics.GetPlayerCharacter` 0)) false false))

(event `self.ReceiveTick`
  (params (DeltaSeconds :type "Float (single-precision)"))
  (bind _returnvalue (`GameplayStatics.GetPlayerCharacter` 0))
  (bind (_returnvalue_roll _returnvalue_pitch _returnvalue_yaw) (`KismetMathLibrary.BreakRotator` (`self.K2_GetActorRotation` _returnvalue)))
  (bind (_returnvalue_x _returnvalue_y) (`KismetMathLibrary.BreakVector` (`self.K2_GetActorLocation` _returnvalue)))
  (`SceneComponent.K2_SetWorldLocationAndRotation` (`self.CaptureComponent2D`) (`KismetMathLibrary.MakeVector` _returnvalue_x _returnvalue_y 1000.0) (`KismetMathLibrary.MakeRotator` 0.0 -90.0 _returnvalue_yaw) false false))

(fn `UserConstructionScript`)